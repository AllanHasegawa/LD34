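; BP_SpriteRepeater is an actor that repeats one Paper2D sprite in a row along its local X axis.
; The construction script calls BuildSprites, which adds NumberOfSprites sprite components, spaces them by StepX, attaches them to the default scene root and assigns Sprite.
; The event graph has no active logic, so the row is built entirely at construction.
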(event EventBeginPlay)

(event EventActorBeginOverlap
  (params (OtherActor :type Actor%20Object%20Reference)))

(event EventTick
  (params (DeltaSeconds :type Float%20%28single-precision%29)))

(fn ConstructionScript
  (CallFunction|BuildSprites))

(fn BuildSprites
  (for _index (range 0 (- (Variables|Default|GetNumber%20of%20Sprites) 1))
    (bind _returnvalue (AddComponent|AddPaperSpriteComponent true (Math|Transform|MakeTransform (Math|Vector|MakeVector (* _index (Variables|Default|GetStep%20X)) 0.0 0.0) "0, 0, 0" "1,1,1")))
    (Class|SceneComponent|Attachto _returnvalue (Variables|Default|GetDefaultSceneRoot) "None" "KeepRelativeOffset" true)
    (Rendering|Components|Sprite|SetSprite _returnvalue (Variables|Default|GetSprite))))