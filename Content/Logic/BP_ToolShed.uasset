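; BP_ToolShed is an actor that lays out a row of tool slots in the level when play begins.
; BuildToolsSlots spawns one BP_ToolSlot per entry in ToolsList, passing that entry as the slot's ToolSlotType.
; Slots start at the actor location plus LocOffset and step along world X by XStep, and each is stored in ToolsSlots.
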(event EventBeginPlay
  (CallFunction|BuildToolsSlots))

(event EventActorBeginOverlap
  (params (OtherActor :type Actor%20Object%20Reference)))

(event EventTick
  (params (DeltaSeconds :type Float%20%28single-precision%29)))

(fn ConstructionScript)

(fn BuildToolsSlots
  (bind _returnvalue (Transformation|GetActorLocation))
  (bind _loc_offset (LocalVariables|GetLoc%20Offset))
  (bind _returnvalue_2 (+ _returnvalue _loc_offset))
  (for (_array_element _array_index) (Variables|Default|GetTools%20List)
    (bind _returnvalue_3 (Game|SpawnActorfromClass "/Game/Logic/BP_ToolSlot.BP_ToolSlot_C" (Math|Transform|MakeTransform (Math|Vector|MakeVector (+ (* _array_index (LocalVariables|GetX%20Step)) (.x _returnvalue_2)) (.y _returnvalue_2) (.z _returnvalue_2)) "0, 0, 0" "1,1,1") "AlwaysSpawn" 0 _array_element 0))
    (Utilities|Array|Add (Variables|Default|GetTools%20Slots) _returnvalue_3)))