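; Main game mode for a farming game, bridging the level's fields, tool shed and player to persistent data in the game instance.
; It equips the saved tool on BeginPlay and spawns the field columns and shed from saved data on request.
; Sleep gathers field and tool-slot state, advances watered crops and clears watering, saves through the game instance, then opens L_Home.
; It also tracks turnip seed counts and stores horizontal camera bounds.
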(event EventBeginPlay
  (bind _asgi (Utilities|Casting|CastToGI (Game|GetGameInstance)))
  (bind _output_get (Variables|Default|SetGI _asgi))
  (bind _equipped_tool (Default|LoadEquippedTool _output_get))
  (bind _asmc (Utilities|Casting|CastToMC (Pawn|GetControlledPawn (.Main%20PC (CallFunction|MainPC)))))
  (bind _output_get_2 (Variables|Default|SetMC _asmc))
  (Default|EquipTool _output_get_2 _equipped_tool))

(event EventTick
  (params (DeltaSeconds :type Float%20%28single-precision%29)))

(fn ConstructionScript)

(fn GetToday
  (return (Variables|/Game/Logic/GI.GI_C|GetToday (Variables|Default|GetGI))))

(fn LoadFieldsDatafromGI
  (params (Start%20Location :type Vector))
  (bind _fields_data (Default|LoadFieldsData (Variables|Default|GetGI)))
  (bind _returnvalue (Game|SpawnActorfromClass "/Game/Logic/Fields/BP_FieldColumnsGroup.BP_FieldColumnsGroup_C" (Math|Transform|MakeTransform Start%20Location "0, 0, 0" "1,1,1") "Undefined" 0 _fields_data 0))
  (Variables|Default|SetFields%20Columns%20Group _returnvalue))

(fn Sleep
  (bind _fields_data (CallFunction|GetFieldsData))
  (bind _processed_fields_data (CallFunction|ProcessWateredFields _fields_data))
  (bind _tools_slots (CallFunction|GetToolsSlots))
  (Default|Sleep (Variables|Default|GetGI) _processed_fields_data _tools_slots (Variables|Default|GetMC))
  (Game|OpenLevel(byName) "L_Home"))

(fn LoadToolShed
  (params (Location :type Vector))
  (bind _tools_slots (Default|LoadToolsSlots (Variables|Default|GetGI)))
  (bind _returnvalue (Game|SpawnActorfromClass "/Game/Logic/BP_ToolShed.BP_ToolShed_C" (Math|Transform|MakeTransform Location "0, 0, 0" "1,1,1") "AlwaysSpawn" 0 _tools_slots 0))
  (Variables|Default|SetTools%20Shed _returnvalue))

(fn SeedsLeft
  (params (Seed%20Type :type BP%20Base%20Field%20Top%20Class%20Reference))
  (bind _gi (Variables|Default|GetGI))
  (bind _number_of_turnip_seeds (Variables|/Game/Logic/GI.GI_C|GetNumber%20of%20Turnip%20Seeds _gi))
  (if (== Seed%20Type "/Game/Logic/Fields/BP_TurnipFieldTop.BP_TurnipFieldTop_C")
    (return _number_of_turnip_seeds (> _number_of_turnip_seeds 0))
    (else
      (return 0 false))))

(fn ConsumeSeed
  (params (Seed%20Type :type BP%20Base%20Field%20Top%20Class%20Reference))
  (bind _gi (Variables|Default|GetGI))
  (if (== Seed%20Type "/Game/Logic/Fields/BP_TurnipFieldTop.BP_TurnipFieldTop_C")
    (Variables|/Game/Logic/GI.GI_C|SetNumber%20of%20Turnip%20Seeds _gi (Math|Integer|Clamp(Integer) (- (Variables|/Game/Logic/GI.GI_C|GetNumber%20of%20Turnip%20Seeds _gi) 1) 0 500))))

(fn GetFieldsData
  (for _array_element (Variables|/Game/Logic/Fields/BP_FieldColumnsGroup.BP_FieldColumnsGroup_C|GetField%20Columns (Variables|Default|GetFields%20Columns%20Group))
    (for _index (range (Default|FirstIndex _array_element) (Default|LastIndex _array_element))
      (Utilities|Array|Add (LocalVariables|GetLoc%20Fields%20Data) (Utilities|Array|Get(acopy) (Variables|/Game/Logic/Fields/BP_FieldColumn.BP_FieldColumn_C|GetFields%20Data _array_element) _index))))
  (return (LocalVariables|GetLoc%20Fields%20Data)))

(fn GetToolsSlots
  (for _array_element (Variables|/Game/Logic/BP_ToolShed.BP_ToolShed_C|GetTools%20Slots (Variables|Default|GetTools%20Shed))
    (Utilities|Array|Add (LocalVariables|GetLoc%20Tools%20Slots) (Variables|/Game/Logic/BP_ToolSlot.BP_ToolSlot_C|GetTool%20Slot%20Type _array_element)))
  (return (LocalVariables|GetLoc%20Tools%20Slots)))

(fn ProcessWateredFields
  (params (Fields%20Data :type Array%20of%20BS%20Field%20Data%20Structures))
  (bind _output_get (LocalVariables|SetLoc%20Fields%20Data Fields%20Data))
  (for (_array_element _array_index) _output_get
    (if (and (.Watered (Utilities|Struct|BreakBS_FieldData _array_element)) (Utilities|IsValid (.OnTop (Utilities|Struct|BreakBS_FieldData _array_element))))
      (LocalVariables|SetNew%20Top%20Days%20With%20Water (+ (.TopDaysWithWater (Utilities|Struct|BreakBS_FieldData _array_element)) 1))
      (else
        (LocalVariables|SetNew%20Top%20Days%20With%20Water (.TopDaysWithWater (Utilities|Struct|BreakBS_FieldData _array_element)))))
    (Utilities|Array|SetArrayElem (LocalVariables|GetLoc%20Fields%20Data) _array_index (Utilities|Struct|MakeBS_FieldData (.ColumIndex (Utilities|Struct|BreakBS_FieldData _array_element)) (.RowIndex (Utilities|Struct|BreakBS_FieldData _array_element)) 0 0 false (.Hoed (Utilities|Struct|BreakBS_FieldData _array_element)) (.OnTop (Utilities|Struct|BreakBS_FieldData _array_element)) (.TopClass (Utilities|Struct|BreakBS_FieldData _array_element)) (LocalVariables|GetNew%20Top%20Days%20With%20Water))))
  (return (LocalVariables|GetLoc%20Fields%20Data)))

(fn SetCameraBounds
  (params (Min :type Actor%20Object%20Reference) (Max :type Actor%20Object%20Reference))
  (Variables|Default|SetCamera%20Bounds (Math|Vector2D|MakeVector2D (.x (Transformation|GetActorLocation Min)) (.x (Transformation|GetActorLocation Max)))))