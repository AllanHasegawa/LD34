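; BP_Enemy is an attackable sprite enemy, configured from an EnemyData struct that supplies its sprite, tint and "Attack" prompt name at construction.
; Each action costs the player one damage and reduces enemy HP by the equipped tool's damage.
; At zero HP or below it reports its Index to the game manager once.
; Tick polls the Alive flag to swap in the tinted dead sprite, deactivate it and disable blocking collision once.
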(event EventDotheAction
  (bind _mc (Variables|Default|GetMC))
  (bind _enemy_data (Variables|Default|GetEnemy%20Data))
  (bind _hp (Utilities|Struct|BreakBS_Enemy _enemy_data))
  (bind _equipped_in_hand (Variables|/Game/Logic/MC.MC_C|GetEquipped%20In%20Hand _mc))
  (bind _damage (CallFunction|ToolTypetoDamage _equipped_in_hand))
  (bind _returnvalue (- _hp _damage))
  (bind _returnvalue_2 (> _returnvalue 0))
  (Default|TakeOneDamage (Variables|/Game/Logic/GM_MainGM.GM_MainGM_C|GetMC (.GM (CallFunction|GM))))
  (bind _structout (Utilities|Struct|SetmembersinBS_Enemy _enemy_data _returnvalue))
  (Utilities|Struct|SetmembersinBS_Enemy _structout _returnvalue_2)
  (if (not _returnvalue_2)
    (Utilities|FlowControl|DoOnce false
      (:Completed
        (Default|ReportEnemyDied (.GM (CallFunction|GM)) (Variables|Default|GetIndex))))))

(event EventTick
  (params (DeltaSeconds :type Float%20%28single-precision%29))
  (bind _enemy_data (Variables|Default|GetEnemy%20Data))
  (if (not (.alive _enemy_data))
    (Utilities|FlowControl|DoOnce false
      (:Completed
        (Sprite|SetSpriteColor (Variables|Default|GetPaperSprite) (* (Variables|Default|GetDead%20sprite%20color) (.spritetone _enemy_data)))
        (Variables|Default|SetActive false)
        (Collision|SetCollisionEnabled (Variables|Default|GetBlocking%20Volume) "NoCollision")
        (Rendering|Components|Sprite|SetSprite (Variables|Default|GetPaperSprite) (.deadsprite (Variables|Default|GetEnemy%20Data)))))))

(fn ConstructionScript
  (bind _papersprite (Variables|Default|GetPaperSprite))
  (bind _enemy_data (Variables|Default|GetEnemy%20Data))
  (|CallParentFunction)
  (Rendering|Components|Sprite|SetSprite _papersprite (.sprite _enemy_data))
  (Sprite|SetSpriteColor _papersprite (.spritetone _enemy_data))
  (Variables|Default|SetAction%20Text (Utilities|Text|ToText(String) (Utilities|String|Append "Attack " (Utilities|String|ToString(Text) (.name _enemy_data)) "!"))))