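; BP_EnemiesSpawner is an actor that spawns a row of enemies from a data list when play begins.
; BuildEnemies spawns one BP_Enemy per EnemiesList entry, passing its index and data, spaced by XStep along world X from the spawner's location plus an offset.
; Spawned actors are kept in EnemiesActorList, from which GetUpdatedEnemiesList collects and returns each enemy's current EnemyData.
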(event EventBeginPlay
  (CallFunction|BuildEnemies))

(fn ConstructionScript)

(fn BuildEnemies
  (bind _returnvalue (Transformation|GetActorLocation))
  (bind _offset (LocalVariables|GetOffset))
  (bind _returnvalue_2 (+ _returnvalue _offset))
  (for (_array_element _array_index) (Variables|Default|GetEnemies%20List)
    (bind _returnvalue_3 (Game|SpawnActorfromClass "/Game/Logic/Enemies/BP_Enemy.BP_Enemy_C" (Math|Transform|MakeTransform (Math|Vector|MakeVector (+ (* _array_index (Variables|Default|GetX%20Step)) (.x _returnvalue_2)) (.y _returnvalue_2) (.z _returnvalue_2)) "0, 0, 0" "1,1,1") "Undefined" 0 _array_index _array_element))
    (Utilities|Array|Add (Variables|Default|GetEnemies%20Actor%20List) _returnvalue_3)))

(fn GetUpdatedEnemiesList
  (for _array_element (Variables|Default|GetEnemies%20Actor%20List)
    (Utilities|Array|Add (LocalVariables|GetRet%20List) (Variables|/Game/Logic/Enemies/BP_Enemy.BP_Enemy_C|GetEnemy%20Data _array_element)))
  (return (LocalVariables|GetRet%20List)))