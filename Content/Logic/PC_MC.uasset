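; PC_MC is the player controller for the MC pawn, handling startup UI and horizontal movement input.
; On BeginPlay it adds the HUD and a new-day widget to the viewport and disables input.
; The new-day widget's closing event re-enables input and sets an EnabledInput flag.
; The Right axis casts the controlled pawn to MC and applies forced movement along world X.
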(event Custom|CB%20NewDay%20Closing_Event_0
  (Input|EnableInput 0)
  (Variables|Default|SetEnabled%20Input true))

(event EventBeginPlay
  (bind _returnvalue (UserInterface|CreateWidget "/Game/UI/W_HUD.W_HUD_C" self))
  (UserInterface|Viewport|AddtoViewport _returnvalue 0)
  (Input|DisableInput 0)
  (bind _returnvalue_2 (UserInterface|CreateWidget "/Game/UI/W_NewDay.W_NewDay_C" self))
  (UserInterface|Viewport|AddtoViewport _returnvalue_2 0)
  (EventDispatchers|AssignNewDayClosing _returnvalue_2 (delegate Custom|CB%20NewDay%20Closing_Event_0)))

(event Input|AxisEvents|InputAxisRight
  (params (AxisValue :type Float%20%28single-precision%29))
  (Pawn|Input|AddMovementInput (.AsMC (Utilities|Casting|CastToMC (Pawn|GetControlledPawn))) (Math|Vector|MakeVector AxisValue 0.0 0.0) 1.0 true))

(fn ConstructionScript)