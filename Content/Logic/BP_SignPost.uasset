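; BP_SignPost is a signpost actor that sends the player to another level.
; On BeginPlay it builds its action text from "Travel to" and the name of the LevelToGo enum value.
; Its DotheAction event passes LevelToGo to the GM's TransitionToAnotherLevel to carry out the travel.
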(event EventBeginPlay
  (Variables|Default|SetAction%20Text (Utilities|Text|ToText(String) (Utilities|String|Append "Travel to " (Utilities|String|EnumtoString (Variables|Default|GetLevel%20to%20Go))))))

(event EventActorBeginOverlap
  (params (OtherActor :type Actor%20Object%20Reference)))

(event EventTick
  (params (DeltaSeconds :type Float%20%28single-precision%29)))

(event EventDotheAction
  (Default|TransitiontoAnotherLevel (.GM (CallFunction|GM)) (Variables|Default|GetLevel%20to%20Go)))

(fn ConstructionScript
  (|CallParentFunction))