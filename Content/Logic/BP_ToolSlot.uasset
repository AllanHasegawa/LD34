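; Tool slot actor that represents a tool, weapon or seed pickup, with a Paper2D sprite and action text chosen by its ToolSlotType.
; On BeginPlay, RefreshAll calls RefreshSprite to set the sprite and RefreshText to build the "Pickup" label from the item name.
; Swords reuse the hoe sprite, and potato seeds, cabbage seeds and Empty have no sprite assigned.
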(event EventBeginPlay
  (CallFunction|RefreshAll))

(event EventActorBeginOverlap
  (params (OtherActor :type Actor%20Object%20Reference)))

(event EventTick
  (params (DeltaSeconds :type Float%20%28single-precision%29)))

(fn ConstructionScript
  (|CallParentFunction))

(fn RefreshSprite
  (Rendering|Components|Sprite|SetSprite (Variables|Default|GetPaperSprite) (Utilities|Select :Index (Variables|Default|GetTool%20Slot%20Type) :NewEnumerator0 "/Game/Graphics/Tools/hoe_512_Sprite.hoe_512_Sprite" :NewEnumerator1 "/Game/Graphics/Tools/watercan_512_Sprite.watercan_512_Sprite" :NewEnumerator2 "/Game/Graphics/Tools/handcart_1024_Sprite.handcart_1024_Sprite" :NewEnumerator3 "/Game/Graphics/Tools/hoe_512_Sprite.hoe_512_Sprite" :NewEnumerator4 "/Game/Graphics/Tools/hoe_512_Sprite.hoe_512_Sprite" :NewEnumerator5 "/Game/Graphics/Tools/hoe_512_Sprite.hoe_512_Sprite" :NewEnumerator7 "/Game/Graphics/Fields/turnip_mature_256_Sprite.turnip_mature_256_Sprite" :NewEnumerator8 0 :NewEnumerator9 0 :NewEnumerator6 0)))

(fn RefreshText
  (Variables|Default|SetAction%20Text (Utilities|Text|ToText(String) (Utilities|String|Append "Pickup " (Utilities|String|MakeLiteralString (Utilities|Select :Index (Variables|Default|GetTool%20Slot%20Type) :NewEnumerator0 "Hoe" :NewEnumerator1 "Watercan" :NewEnumerator2 "Handcart" :NewEnumerator3 "Wooden Sword" :NewEnumerator4 "Iron Sword" :NewEnumerator5 "+10 Diamon Sword" :NewEnumerator7 "Turnip Seeds" :NewEnumerator8 "Potato Seeds" :NewEnumerator9 "Cabbage Seeds" :NewEnumerator6 ""))))))

(fn RefreshAll
  (CallFunction|RefreshSprite)
  (CallFunction|RefreshText))