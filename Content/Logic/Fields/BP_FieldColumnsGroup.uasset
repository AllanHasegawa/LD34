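; BP_FieldColumnsGroup is an actor that builds and owns a row of BP_FieldColumn actors at runtime.
; On BeginPlay it spawns one column per NumberOfColumns, spaced by XStep along world X from its own location.
; Each column receives its index and the shared FieldsData, attaches to the group's root, and is stored in FieldColumns.
; It then tells every stored column to update its sprites.
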(event EventBeginPlay
  (CallFunction|BuildFieldColumns)
  (CallFunction|UpdateAllSprites))

(event EventActorBeginOverlap
  (params (OtherActor :type Actor%20Object%20Reference)))

(event EventTick
  (params (DeltaSeconds :type Float%20%28single-precision%29)))

(fn ConstructionScript)

(fn BuildFieldColumns
  (bind _returnvalue (Transformation|GetActorLocation))
  (for _index (range 0 (- (CallFunction|NumberOfColumns) 1))
    (bind _returnvalue_2 (Game|SpawnActorfromClass "/Game/Logic/Fields/BP_FieldColumn.BP_FieldColumn_C" (Math|Transform|MakeTransform (Math|Vector|MakeVector (+ (.x _returnvalue) (* _index (LocalVariables|GetX%20Step))) (.y _returnvalue) (.z _returnvalue)) "0, 0, 0" "1,1,1") "AlwaysSpawn" 0 _index (Variables|Default|GetFields%20Data)))
    (Class|Actor|AttachRootComponentto _returnvalue_2 (Variables|Default|GetDefaultSceneRoot) "None" "KeepWorldPosition" true)
    (Utilities|Array|Add (Variables|Default|GetField%20Columns) _returnvalue_2)))

(fn UpdateAllSprites
  (for _array_element (Variables|Default|GetField%20Columns)
    (Default|UpdateAllSprites _array_element)))