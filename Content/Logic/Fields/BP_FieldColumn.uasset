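; One column of farm plots that can be watered, hoed and seeded as a whole.
; On BeginPlay it builds soil and hoe-mark sprites per row and respawns crop actors from FieldsData, a flattened 2D array indexed by column and row.
; Water, Hoe and Seed update that column's slice, stamping game days and spawning crops on empty plots, then refresh sprites.
; DotheAction runs all three, planting turnips.
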(event EventDotheAction
  (CallFunction|Water)
  (CallFunction|Hoe)
  (CallFunction|Seed "/Game/Logic/Fields/BP_TurnipFieldTop.BP_TurnipFieldTop_C"))

(event EventBeginPlay
  (CallFunction|Rebuild)
  (CallFunction|UpdateAllSprites))

(event EventActorBeginOverlap
  (params (OtherActor :type Actor%20Object%20Reference)))

(event EventTick
  (params (DeltaSeconds :type Float%20%28single-precision%29)))

(fn ConstructionScript
  (|CallParentFunction))

(fn Rebuild
  (for _index (range 0 (- (CallFunction|NumberOfRows) 1))
    (bind _returnvalue (AddComponent|AddPaperSpriteComponent true (Math|Transform|MakeTransform (Math|Vector|MakeVector 0.0 0.0 (* _index (LocalVariables|GetInterval%20Step))) "0, 0, 0" (Math|Conversions|ToVector(Float) 0.2))))
    (Class|SceneComponent|Attachto _returnvalue (Variables|Default|GetPaperSprite) "None" "KeepRelativeOffset" true)
    (bind _returnvalue_2 (AddComponent|AddPaperSpriteComponent true (Math|Transform|MakeTransform (Math|Vector|MakeVector 0.0 1e+01 (* _index (LocalVariables|GetInterval%20Step))) "0, 0, 0" (Math|Conversions|ToVector(Float) 0.2))))
    (Class|SceneComponent|Attachto _returnvalue_2 (Variables|Default|GetPaperSprite) "None" "KeepRelativeOffset" true)
    (bind _top_actor (CallFunction|RebuildTopActor (.topclass (Utilities|Array|Get(acopy) (Variables|Default|GetFields%20Data) (CallFunction|2Dto1D (Variables|Default|GetColumn%20Index) _index))) (.topdaycreated (Utilities|Array|Get(acopy) (Variables|Default|GetFields%20Data) (CallFunction|2Dto1D (Variables|Default|GetColumn%20Index) _index))) _returnvalue))
    (Utilities|Array|SetArrayElem (Variables|Default|GetFields%20Data) (CallFunction|2Dto1D (Variables|Default|GetColumn%20Index) _index) (Utilities|Struct|MakeBS_FieldData (.columindex (Utilities|Array|Get(acopy) (Variables|Default|GetFields%20Data) (CallFunction|2Dto1D (Variables|Default|GetColumn%20Index) _index))) (.rowindex (Utilities|Array|Get(acopy) (Variables|Default|GetFields%20Data) (CallFunction|2Dto1D (Variables|Default|GetColumn%20Index) _index))) _returnvalue _returnvalue_2 (.watered (Utilities|Array|Get(acopy) (Variables|Default|GetFields%20Data) (CallFunction|2Dto1D (Variables|Default|GetColumn%20Index) _index))) (.hoed (Utilities|Array|Get(acopy) (Variables|Default|GetFields%20Data) (CallFunction|2Dto1D (Variables|Default|GetColumn%20Index) _index))) _top_actor (.topclass (Utilities|Array|Get(acopy) (Variables|Default|GetFields%20Data) (CallFunction|2Dto1D (Variables|Default|GetColumn%20Index) _index))) (.topdaycreated (Utilities|Array|Get(acopy) (Variables|Default|GetFields%20Data) (CallFunction|2Dto1D (Variables|Default|GetColumn%20Index) _index))) (.lastdaywatered (Utilities|Array|Get(acopy) (Variables|Default|GetFields%20Data) (CallFunction|2Dto1D (Variables|Default|GetColumn%20Index) _index)))))))

(fn UpdateSingleSprite
  (params (Field%20Data :type BS%20Field%20Data%20Structure))
  (Rendering|Components|Sprite|SetSprite (.sprite Field%20Data) (select (.watered Field%20Data) "/Game/Graphics/Fields/field_wet_256_Sprite.field_wet_256_Sprite" "/Game/Graphics/Fields/field_256_Sprite.field_256_Sprite"))
  (Rendering|Components|Sprite|SetSprite (.hoemarkssprite Field%20Data) "/Game/Graphics/Fields/field_rack_256_Sprite.field_rack_256_Sprite")
  (Rendering|SetVisibility (.hoemarkssprite Field%20Data) (.hoed Field%20Data) true))

(fn UpdateAllSprites
  (for _index (range (CallFunction|FirstIndex) (CallFunction|LastIndex))
    (CallFunction|UpdateSingleSprite (Utilities|Array|Get(acopy) (Variables|Default|GetFields%20Data) _index))))

(fn Hoe
  (for _index (range (CallFunction|FirstIndex) (CallFunction|LastIndex))
    (Utilities|Array|SetArrayElem (Variables|Default|GetFields%20Data) _index (Utilities|Struct|MakeBS_FieldData (.columindex (Utilities|Array|Get(acopy) (Variables|Default|GetFields%20Data) _index)) (.rowindex (Utilities|Array|Get(acopy) (Variables|Default|GetFields%20Data) _index)) (.sprite (Utilities|Array|Get(acopy) (Variables|Default|GetFields%20Data) _index)) (.hoemarkssprite (Utilities|Array|Get(acopy) (Variables|Default|GetFields%20Data) _index)) (.watered (Utilities|Array|Get(acopy) (Variables|Default|GetFields%20Data) _index)) true (.ontop (Utilities|Array|Get(acopy) (Variables|Default|GetFields%20Data) _index)) (.topclass (Utilities|Array|Get(acopy) (Variables|Default|GetFields%20Data) _index)) (.topdaycreated (Utilities|Array|Get(acopy) (Variables|Default|GetFields%20Data) _index)) (.lastdaywatered (Utilities|Array|Get(acopy) (Variables|Default|GetFields%20Data) _index))))
    (Utilities|IsValid (.ontop (Utilities|Array|Get(acopy) (Variables|Default|GetFields%20Data) _index))
      (:Is%20Valid
        (Default|Hoe (.ontop (Utilities|Array|Get(acopy) (Variables|Default|GetFields%20Data) _index))))))
  (CallFunction|UpdateAllSprites))

(fn Water
  (for _index (range (CallFunction|FirstIndex) (CallFunction|LastIndex))
    (Utilities|Array|SetArrayElem (Variables|Default|GetFields%20Data) _index (Utilities|Struct|MakeBS_FieldData (.columindex (Utilities|Array|Get(acopy) (Variables|Default|GetFields%20Data) _index)) (.rowindex (Utilities|Array|Get(acopy) (Variables|Default|GetFields%20Data) _index)) (.sprite (Utilities|Array|Get(acopy) (Variables|Default|GetFields%20Data) _index)) (.hoemarkssprite (Utilities|Array|Get(acopy) (Variables|Default|GetFields%20Data) _index)) true (.hoed (Utilities|Array|Get(acopy) (Variables|Default|GetFields%20Data) _index)) (.ontop (Utilities|Array|Get(acopy) (Variables|Default|GetFields%20Data) _index)) (.topclass (Utilities|Array|Get(acopy) (Variables|Default|GetFields%20Data) _index)) (.topdaycreated (Utilities|Array|Get(acopy) (Variables|Default|GetFields%20Data) _index)) (Default|GetToday (.GM (CallFunction|GM))))))
  (CallFunction|UpdateAllSprites))

(fn Seed
  (params (Seed%20Type :type BP%20Base%20Field%20Top%20Class%20Reference))
  (bind _gm (CallFunction|GM))
  (bind _today (Default|GetToday _gm))
  (LocalVariables|SetTopping%20Class Seed%20Type)
  (for _index (range (CallFunction|FirstIndex) (CallFunction|LastIndex))
    (Utilities|IsValid (.ontop (Utilities|Array|Get(acopy) (Variables|Default|GetFields%20Data) _index))
      (:Is%20Not%20Valid
        (bind _top_actor (CallFunction|RebuildTopActor (LocalVariables|GetTopping%20Class) _today (.sprite (Utilities|Array|Get(acopy) (Variables|Default|GetFields%20Data) _index))))
        (Utilities|Array|SetArrayElem (Variables|Default|GetFields%20Data) _index (Utilities|Struct|MakeBS_FieldData (.columindex (Utilities|Array|Get(acopy) (Variables|Default|GetFields%20Data) _index)) (.rowindex (Utilities|Array|Get(acopy) (Variables|Default|GetFields%20Data) _index)) (.sprite (Utilities|Array|Get(acopy) (Variables|Default|GetFields%20Data) _index)) (.hoemarkssprite (Utilities|Array|Get(acopy) (Variables|Default|GetFields%20Data) _index)) (.watered (Utilities|Array|Get(acopy) (Variables|Default|GetFields%20Data) _index)) (.hoed (Utilities|Array|Get(acopy) (Variables|Default|GetFields%20Data) _index)) _top_actor (LocalVariables|GetTopping%20Class) _today (.lastdaywatered (Utilities|Array|Get(acopy) (Variables|Default|GetFields%20Data) _index)))))))
  (CallFunction|UpdateAllSprites))

(fn FirstIndex
  (return (CallFunction|2Dto1D (Variables|Default|GetColumn%20Index))))

(fn LastIndex
  (return (CallFunction|2Dto1D (Variables|Default|GetColumn%20Index) (- (CallFunction|NumberOfRows) 1))))

(fn RebuildTopActor
  (params (Top%20Class :type BP%20Base%20Field%20Top%20Class%20Reference) (Day%20Planted :type Integer) (Field%20Sprite :type Paper%20Sprite%20Component%20Object%20Reference))
  (bind _returnvalue (Transformation|GetWorldTransform Field%20Sprite))
  (if (Utilities|IsValidClass Top%20Class)
    (bind _returnvalue_2 (Game|SpawnActorfromClass Top%20Class (Math|Transform|MakeTransform (+ (.location _returnvalue) (LocalVariables|GetChild%20Topping%20Offset)) (.rotation _returnvalue) (.scale _returnvalue)) "AlwaysSpawn" 0 Day%20Planted 0))
    (Utilities|IsValid _returnvalue_2
      (:Is%20Valid
        (Class|Actor|AttachRootComponentto _returnvalue_2 Field%20Sprite "None" "KeepWorldPosition" false)
        (return _returnvalue_2))
      (:Is%20Not%20Valid
        (return 0)))
    (else
      (return 0))))