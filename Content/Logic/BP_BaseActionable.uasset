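; BP_BaseActionable is a base Blueprint for interactable objects that offer an action prompt when the MC overlaps their box.
; If the MC's CheckAction approves, it creates a W_ActionUI widget with its text and background color, and closes it when overlap ends.
; The widget's callback runs DoTheAction, which only prints a red "Non implemented" warning here, as a placeholder for child classes to override.
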(event OnComponentBeginOverlap(Box)
  (params (OtherActor :type Actor%20Object%20Reference) (OtherComp :type Primitive%20Component%20Object%20Reference) (OtherBodyIndex :type Integer) (bFromSweep :type Boolean) (SweepResult :type Hit%20Result%20Structure%20%28by%20ref%29))
  (bind _asmc (Utilities|Casting|CastToMC OtherActor))
  (bind _output_get (Variables|Default|SetMC _asmc))
  (bind _allow_action (Default|CheckAction _output_get self))
  (if _allow_action
    (bind _returnvalue (UserInterface|CreateWidget "/Game/UI/W_ActionUI.W_ActionUI_C" (.Main%20PC (CallFunction|MainPC)) (Variables|Action|GetAction%20Text) (Variables|Action|GetAction%20Background%20Color)))
    (bind _output_get_2 (Variables|Default|SetW%20Action _returnvalue))
    (EventDispatchers|AssignActionUIDotheAction _output_get_2 (delegate Custom|CB%20ActionUI%20Do%20The%20Action_Event_0))
    (UserInterface|Viewport|AddtoViewport _output_get_2 0)))

(event OnComponentEndOverlap(Box)
  (params (OtherActor :type Actor%20Object%20Reference) (OtherComp :type Primitive%20Component%20Object%20Reference) (OtherBodyIndex :type Integer))
  (bind _w_action (Variables|Default|GetW%20Action))
  (Utilities|Casting|CastToMC OtherActor)
  (Utilities|IsValid _w_action
    (:Is%20Valid
      (Default|Close _w_action))))

(event Custom|Do%20The%20Action
  (Development|PrintString "BaseActionable: Non implemented" true true "(R=1.000000,G=0.000000,B=0.000000,A=1.000000)" 2e+01))

(event Custom|CB%20ActionUI%20Do%20The%20Action_Event_0
  (CallFunction|DotheAction))

(fn ConstructionScript)