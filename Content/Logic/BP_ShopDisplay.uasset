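; Shop display actor that sells one configured tool, sword or seed bundle through an action event.
; Construction script sets the sprite, buy prompt and cost text from the Tool enum, plus a quantity label for seeds.
; At BeginPlay it asks GM to tint and deactivate itself if the sword is already owned or unaffordable.
; Buying goes through GM, and only swords then switch to the owned state.
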(event EventBeginPlay
  (Utilities|FlowControl|Sequence
    (:then_0
      ;[1 1 1] Check if owned
      (switch Utilities|FlowControl|Switch|SwitchonE_ToolSlotType (Variables|Default|GetTool)
        (:NewEnumerator3
          _)
        (:NewEnumerator4
          _)
        (:NewEnumerator5
          _))
      (bind _yes (Default|HasEquipment (.GM (CallFunction|GM)) (Variables|Default|GetTool)))
      (if _yes
        (CallFunction|SetasOwned)))
    (:then_1
      ;[1 1 1] Not enough gold
      (if (not (Default|CanBuyEquipment? (.GM (CallFunction|GM)) (Variables|Default|GetTool) (Variables|Default|GetNumber%20of%20Seeds)))
        (Sprite|SetSpriteColor (Variables|Default|GetItem%20On%20Display%20Sprite) (Variables|Default|GetDisabled%20Color%20Tint))
        (Variables|Default|SetActive false)))))

(event EventDotheAction
  (Default|BuyEquipment (.GM (CallFunction|GM)) (Variables|Default|GetTool) (Variables|Default|GetNumber%20of%20Seeds))
  (switch Utilities|FlowControl|Switch|SwitchonE_ToolSlotType (Variables|Default|GetTool)
    (:NewEnumerator3
      _)
    (:NewEnumerator4
      _)
    (:NewEnumerator5
      _))
  (CallFunction|SetasOwned))

(fn ConstructionScript
  (bind _tool (Variables|Default|GetTool))
  (|CallParentFunction)
  (Rendering|Components|Sprite|SetSprite (Variables|Default|GetItem%20On%20Display%20Sprite) (CallFunction|ToolTypetoSprite _tool))
  (Variables|Default|SetAction%20Text (Utilities|Text|ToText(String) (Utilities|String|Append "Buy " (CallFunction|ToolTypetoString _tool))))
  (Rendering|Components|TextRender|SetText (Variables|Default|GetCost%20Text) (Utilities|Text|ToText(String) (Utilities|String|Append (Utilities|String|ToString(Integer) (CallFunction|ToolTypetoCost (Variables|Default|GetTool))) "G")))
  (Utilities|FlowControl|Sequence
    (:then_0
      (switch Utilities|FlowControl|Switch|SwitchonE_ToolSlotType (Variables|Default|GetTool)
        (:NewEnumerator7
          _)
        (:NewEnumerator8
          _)
        (:NewEnumerator9
          _))
      (Rendering|Components|TextRender|SetText (Variables|Default|GetTimes%20Text) (Utilities|Text|ToText(String) (Utilities|String|Append (Utilities|String|ToString(Integer) (Variables|Default|GetNumber%20of%20Seeds)) "x")))
      (Rendering|SetVisibility (Variables|Default|GetTimes%20Text) true true))))

(fn SetasOwned
  (Sprite|SetSpriteColor (Variables|Default|GetItem%20On%20Display%20Sprite) (Variables|Default|GetDisabled%20Color%20Tint))
  (Rendering|Components|TextRender|SetText (Variables|Default|GetCost%20Text) (Variables|Default|GetAlready%20Owned%20Text))
  (Variables|Default|SetActive false)
  (return))